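; BP_PlayerCart is a player-controlled physics cart driven like a tank, with separate left and right wheel forces.
; BeginPlay adds the CartInput Enhanced Input mapping context for player 0.
; Forward/backward and turning actions share one path that mixes input values by sum and difference into clamped per-side forces.
; These are scaled and applied to PlayerMesh at each wheel location; releasing input zeroes the stored values.
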(event `self.ReceiveBeginPlay`
  ;[0.7656 0.7565 0 0.5] Enhaced Input Player
  (`EnhancedInputSubsystemInterface.AddMappingContext` (pcsubsystem `EnhancedInputLocalPlayerSubsystem` (`GameplayStatics.GetPlayerController` 0)) "/Game/input/CartInput.CartInput" 0 (struct)))

(event `EnhancedInput|/Game/input/IA_ForwardBackward`
  (params (ActionValue :type "Float (double-precision)") (ElapsedSeconds :type "Float (double-precision)") (TriggeredSeconds :type "Float (double-precision)") (InputAction :type "InputAction Object Reference" :default "/Game/input/IA_ForwardBackward.IA_ForwardBackward"))
  (bind _playermesh (`self.PlayerMesh`))
  ;[0.001581 0.15 0.006557 0.5] Симуляция физики колёс и управление
  (:`Triggered`
    (bind _output_get (set `self.LeftWheelForce` (`KismetMathLibrary.FClamp` (+ (stale `EnhancedInput|/Game/input/IA_Turning` ActionValue) ActionValue) -1.0) :!label _label))
    (bind _output_get_2 (set `self.RightWheelForce` (`KismetMathLibrary.FClamp` (- ActionValue (stale `EnhancedInput|/Game/input/IA_Turning` ActionValue)) -1.0)))
    (`PrimitiveComponent.AddForceAtLocationLocal` _playermesh (`KismetMathLibrary.MakeVector` (* _output_get (`self.ForceMultiplier`))) (`SceneComponent.RelativeLocation` (`self.LeftWheels`)) "None")
    (`PrimitiveComponent.AddForceAtLocationLocal` _playermesh (`KismetMathLibrary.MakeVector` (* _output_get_2 (`self.ForceMultiplier`))) (`SceneComponent.RelativeLocation` (`self.RightWheels`)) "None"))
  (:`Completed`
    (set `self.LeftWheelForce` 0.0 :!label _label_2)
    (set `self.RightWheelForce` 0.0)))

(event `EnhancedInput|/Game/input/IA_Turning`
  (params (ActionValue :type "Float (double-precision)") (ElapsedSeconds :type "Float (double-precision)") (TriggeredSeconds :type "Float (double-precision)") (InputAction :type "InputAction Object Reference" :default "/Game/input/IA_Turning.IA_Turning"))
  ;[0.001581 0.15 0.006557 0.5] Симуляция физики колёс и управление
  (:`Triggered`
    (goto _label))
  (:`Completed`
    (goto _label_2)))

(event `self.ReceiveTick`
  (params (DeltaSeconds :type "Float (single-precision)"))
  ;[0 0.15 0.04758 0.5] Отладка колёс
)

(fn `UserConstructionScript`)